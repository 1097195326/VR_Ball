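; BallPawn is a pawn that rolls a physics ball by applying torque scaled by RunSpeed, with VR and non-VR control.
; In VR, Tick copies the right motion controller's yaw to control rotation, and held right or left inputs torque the ball forward or backward around that heading's right vector.
; Those presses also label a text render, while outside VR the movement axes apply world-axis torque.
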(event `InputAction|RightMotionTaked`
  (params (Key :type "Key Structure" :default "AnyKey"))
  (:`Pressed`
    (set `self.MotionFire` true)
    (set `self.ForB` 1)
    (set `self.RenderText` "Right")
    (`TextRenderComponent.K2_SetText` (`self.TextRender`) (`self.RenderText`) :!label _label))
  (:`Released`
    (set `self.MotionFire` false)
    (set `self.ForB` 0)))

(event `InputAction|LeftMotionTaked`
  (params (Key :type "Key Structure" :default "AnyKey"))
  (:`Pressed`
    (set `self.MotionFire` true)
    (set `self.ForB` -1)
    (set `self.RenderText` "Left")
    (goto _label))
  (:`Released`
    (set `self.MotionFire` false)
    (set `self.ForB` 0)))

(event `self.ReceiveTick`
  (params (DeltaSeconds :type "Float (single-precision)"))
  (if (`self.IsVR`)
    (`Controller.SetControlRotation` (`GameplayStatics.GetPlayerController` 0) (`KismetMathLibrary.MakeRotator` 0.0 0.0 (.yaw (`SceneComponent.K2_GetComponentRotation` (`self.RightMotionController`)))))
    (if (`self.MotionFire`)
      (`PrimitiveComponent.AddTorque` (`self.Ball`) (* (* (`KismetMathLibrary.GetRightVector` (`KismetMathLibrary.MakeRotator` 0.0 0.0 (.yaw (`Controller.GetControlRotation` (`GameplayStatics.GetPlayerController` 0))))) (`self.RunSpeed`)) (`self.ForB`)) "None" false))))

(event `InputAxis|MoveForward`
  (params (AxisValue :type "Float (single-precision)"))
  (if (not (`self.IsVR`))
    (`PrimitiveComponent.AddTorque` (`self.Ball`) (`KismetMathLibrary.MakeVector` 0.0 (* AxisValue (`self.RunSpeed`))) "None" false)))

(event `InputAxis|MoveRight`
  (params (AxisValue :type "Float (single-precision)"))
  (if (not (`self.IsVR`))
    (`PrimitiveComponent.AddTorque` (`self.Ball`) (`KismetMathLibrary.MakeVector` (* AxisValue (`self.RunSpeed`) -1.0)) "None" false)))

(fn `UserConstructionScript`)