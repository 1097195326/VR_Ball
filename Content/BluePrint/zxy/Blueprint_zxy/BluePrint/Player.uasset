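; Player Blueprint that rolls its physics body with torque, supporting both VR and non-VR control, and clicks widgets through a WidgetInteraction component.
; In VR, Tick copies the left controller's rotation to control rotation and, while MotionFire is set, applies torque around its right vector.
; Outside VR, movement axes apply world-axis torque scaled by RunSpeed.
; Right mouse and left trigger press the widget pointer, but only trigger release releases it.
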(event `Key|RightMouseButton`
  (params (Key :type "Key Structure" :default "AnyKey"))
  (:`Pressed`
    (`WidgetInteractionComponent.PressPointerKey` (`self.WidgetInteraction`) "LeftMouseButton" :!label _label)))

(event `Key|MotionController_Left_Trigger`
  (params (Key :type "Key Structure" :default "AnyKey"))
  (:`Pressed`
    (`|ExecutionSequence`
      (:`then_0`
        (goto _label))))
  (:`Released`
    (`WidgetInteractionComponent.ReleasePointerKey` (`self.WidgetInteraction`) "LeftMouseButton")))

(event `self.ReceiveTick`
  (params (DeltaSeconds :type "Float (single-precision)"))
  ;[1 0.2916 0.3015] 注释
  (if (`self.IsVR`)
    (`Controller.SetControlRotation` (`GameplayStatics.GetPlayerController` 0) (`KismetMathLibrary.MakeRotator` (.roll (`SceneComponent.K2_GetComponentRotation` (`self.LeftMotionController`))) (.pitch (`SceneComponent.K2_GetComponentRotation` (`self.LeftMotionController`))) (.yaw (`SceneComponent.K2_GetComponentRotation` (`self.LeftMotionController`)))))
    (if (`self.MotionFire`)
      (`PrimitiveComponent.AddTorque` (`self.Player`) (* (* (`KismetMathLibrary.GetRightVector` (`Controller.GetControlRotation` (`GameplayStatics.GetPlayerController` 0))) (`self.RunSpeed`)) (`self.ForB`)) "None" false))))

(event `InputAxis|MoveForward`
  (params (AxisValue :type "Float (single-precision)"))
  ;[1 1 1] 移动
  (if (not (`self.IsVR`))
    (`PrimitiveComponent.AddTorque` (`self.Player`) (`KismetMathLibrary.MakeVector` 0.0 (* AxisValue (`self.RunSpeed`))) "None" false)))

(event `InputAxis|MoveRight`
  (params (AxisValue :type "Float (single-precision)"))
  ;[1 1 1] 移动
  (if (not (`self.IsVR`))
    (`PrimitiveComponent.AddTorque` (`self.Player`) (`KismetMathLibrary.MakeVector` (* AxisValue (`self.RunSpeed`) -1.0)) "None" false)))

(fn `UserConstructionScript`)