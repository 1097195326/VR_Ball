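; BallPawn is a pawn that the player rolls around as a physics ball.
; Turn and LookUp axes drive controller yaw and pitch, while Forward applies Strength-scaled torque around the camera yaw's right vector to roll the ball forward or back.
; No sideways input is wired, Tick is empty, and leftover motion-controller steering nodes, which feed world Z location in as yaw, never run.
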(event `InputAxis|turn`
  (params (AxisValue :type "Float (single-precision)"))
  ;[1 1 1] 四周看
  (`self.AddControllerYawInput` AxisValue))

(event `InputAxis|LookUp`
  (params (AxisValue :type "Float (single-precision)"))
  ;[1 1 1] 四周看
  (`self.AddControllerPitchInput` AxisValue))

(event `InputAxis|Forward`
  (params (AxisValue :type "Float (single-precision)"))
  ;[1 1 1] 前后
  (`PrimitiveComponent.AddTorque` (`self.Ball`) (* (`KismetMathLibrary.GetRightVector` (`KismetMathLibrary.MakeRotator` 0.0 0.0 (.yaw (`SceneComponent.GetSocketRotation` (`self.Camera`) "None")))) (* AxisValue (`self.Strength`))) "None" false))

(event `self.ReceiveTick`
  (params (DeltaSeconds :type "Float (single-precision)"))
  ;[1 1 1] 注释
)

(fn `UserConstructionScript`)